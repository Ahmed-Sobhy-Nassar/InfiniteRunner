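; Runner character Blueprint that handles lane switching and an unfinished distance tracker intended to increase speed over distance.
; ChangeLane plays a timeline, feeding its lane value to ChangeLaneUpdate and calling ChangeLaneFinished on completion, neither of which is defined in this Blueprint.
; GetDistance_1 adds movement since the last stored location to a running total, then ends on a short delay without looping or changing speed.
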(event `GetDistance_1`
  ;[1 0.1214 0.2714] Trying to get the distance traveled to increase the speed, NOT FINISHED YET
  (set `self.DistanceTravled` (+ (`KismetMathLibrary.VSize` (- (`self.Location`) (`self.K2_GetActorLocation`))) (`self.DistanceTravled`)))
  (set `self.Location` (`self.K2_GetActorLocation`))
  (`KismetSystemLibrary.Delay` 0.2))

(event `self.ChangeLane`
  (bind (_direction _lanevalue) (`Timeline|LaneSwithingTimeLine` :!via `PlayFromStart`)
    (:`Update`
      (`self.ChangeLaneUpdate` _lanevalue))
    (:`Finished`
      (`self.ChangeLaneFinished`))))

(fn `UserConstructionScript`)